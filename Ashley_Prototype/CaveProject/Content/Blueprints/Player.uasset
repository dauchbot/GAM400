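; Player Blueprint for a physics sphere moved in the X-Z plane, with health and checkpoint respawn.
; Each tick, axis input accelerates a stored velocity, which is capped at max speed, written to the sphere and damped by per-frame drag.
; Hitting a VerticalEnemy adds knockback along the hit normal and costs health.
; At zero health, Die teleports the player to the checkpoint recorded at BeginPlay and restores health.
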(event `self.ReceiveBeginPlay`
  (`self.EnableInput` (`GameplayStatics.GetPlayerController` 0))
  (set `self.CheckpointLocation` (`self.K2_GetActorLocation`)))

(event `self.ReceiveActorBeginOverlap`
  (params (OtherActor :type "Actor Object Reference")))

(event `self.ReceiveTick`
  (params (DeltaSeconds :type "Float (single-precision)"))
  (bind _returnvalue (`GameplayStatics.GetWorldDeltaSeconds`))
  (bind _acceleration (`self.Acceleration`))
  (bind _maxspeed (`self.MaxSpeed`))
  (bind _output_get (set `self.Velocity` (+ (`self.Velocity`) (`KismetMathLibrary.MakeVector` (* (`self.GetInputAxisValue`) _acceleration _returnvalue) 0.0 (* (`self.GetInputAxisValue`) _acceleration _returnvalue)))))
  (if (> (`KismetMathLibrary.VSizeSquared` _output_get) (* _maxspeed _maxspeed))
    (set `self.Velocity` (* (`KismetMathLibrary.Normal` (`self.Velocity`)) (`self.MaxSpeed`))))
  (`PrimitiveComponent.SetPhysicsLinearVelocity` (`self.Sphere`) (`self.Velocity`) false "None")
  (set `self.Velocity` (* (`self.Velocity`) (`self.Drag`))))

(event `self.ReceiveHit`
  (params (MyComp :type "PrimitiveComponent Object Reference") (Other :type "Actor Object Reference") (OtherComp :type "PrimitiveComponent Object Reference") (bSelfMoved :type Boolean) (HitLocation :type "Vector Structure") (HitNormal :type "Vector Structure") (NormalImpulse :type "Vector Structure") (Hit :type "HitResult Structure (by ref)"))
  (if (== (`GameplayStatics.GetObjectClass` Other) "/Game/Blueprints/VerticalEnemy.VerticalEnemy_C")
    (set `self.Velocity` (+ (`self.Velocity`) (* HitNormal (`self.Knockback`))))
    (`/Engine/EditorBlueprintResources/StandardMacros.DecrementInt` (`self.Health`)
      (:`  `
        (if (<= (`self.Health`) 0)
          (`self.Die`))))))

(fn `Die`
  (`PrimitiveComponent.SetPhysicsLinearVelocity` (`self.Sphere`) (0.0 0.0 0.0) false "None")
  (`self.K2_SetActorLocation` (`self.CheckpointLocation`))
  (set `self.Health` (`self.MaxHealth`)))

(fn `UserConstructionScript`)
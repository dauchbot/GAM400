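; VerticalEnemy is an enemy actor that patrols up and down along the world Z axis around its spawn location.
; BeginPlay records the start position, and Tick moves the actor by MoveSpeed scaled by delta time without sweeping.
; A MovingUp flag flips whenever the actor passes MovementRadius above or below that start height, producing a continuous ping-pong motion.
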(event `self.ReceiveBeginPlay`
  (set `self.StartPosition` (`self.K2_GetActorLocation`)))

(event `self.ReceiveActorBeginOverlap`
  (params (OtherActor :type "Actor Object Reference")))

(event `self.ReceiveTick`
  (params (DeltaSeconds :type "Float (single-precision)"))
  (if (`self.MovingUp`)
    (`self.K2_AddActorWorldOffset` (`KismetMathLibrary.MakeVector` 0.0 0.0 (* (`self.MoveSpeed`) (`GameplayStatics.GetWorldDeltaSeconds`))))
    (if (> (.z (`self.K2_GetActorLocation`)) (+ (.z (`self.StartPosition`)) (`self.MovementRadius`)))
      (set `self.MovingUp` false))
    (else
      (`self.K2_AddActorWorldOffset` (`KismetMathLibrary.MakeVector` 0.0 0.0 (* (`self.MoveSpeed`) (`GameplayStatics.GetWorldDeltaSeconds`) -1.0)))
      (if (< (.z (`self.K2_GetActorLocation`)) (- (.z (`self.StartPosition`)) (`self.MovementRadius`)))
        (set `self.MovingUp` true)))))

(fn `UserConstructionScript`)